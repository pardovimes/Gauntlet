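; BP_Spider is a spider enemy with health and a floating health bar.
; On BeginPlay it links its WBP_HealthBar widget to itself and colors the bar red.
; Damage lowers Health while the spider is alive; once it dies, the actor waits a few seconds for the death animation, then destroys itself.
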(event `self.ReceiveBeginPlay`
  (bind _aswbp_health_bar (cast `/Game/UI/WBP_HealthBar` (`WidgetComponent.GetUserWidgetObject` (`self.HealthBar`))))
  (set `/Game/UI/WBP_HealthBar.Character` self _aswbp_health_bar)
  (set `/Game/UI/WBP_HealthBar.LifeColor` (struct :`R` 1.0 :`A` 1.0) _aswbp_health_bar))

(event `self.ReceiveAnyDamage`
  (params (Damage :type "Float (single-precision)") (DamageType :type "DamageType Object Reference") (InstigatedBy :type "Controller Object Reference") (DamageCauser :type "Actor Object Reference"))
  ;[1 1 1] If it's not dead we decrease the life
  (if (not (`self.isDead`))
    (set `self.health` (- (`self.health`) Damage))
    ;[1 1 1] If spider is dead in 5 seconds destroy (to show the animation)
    (if (`self.isDead`)
      (`KismetSystemLibrary.Delay` 5.0)
      (`self.K2_DestroyActor`))))

(fn `UserConstructionScript`)